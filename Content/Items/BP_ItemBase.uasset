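; Base actor for world item pickups that go into the player's inventory on touch.
; On BeginPlay, a missing ItemObject is filled from GetDefaultItemObject, which is empty in this base, and the root is re-set to its current location.
; Sphere overlap with a PlayerCharacter passes the ItemObject to InventoryComponent.TryAddItem, and the actor destroys itself only if that succeeds.
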(event `self.ReceiveBeginPlay`
  (bind (_returnvalue_x _returnvalue_y _returnvalue_z) (`KismetMathLibrary.BreakVector` (`SceneComponent.K2_GetComponentLocation` (`self.DefaultSceneRoot`))))
  (if (not (`KismetSystemLibrary.IsValid` (`self.ItemObject`)))
    (bind _itemobject (`self.GetDefaultItemObject`))
    (set `self.ItemObject` _itemobject)
    (`SceneComponent.K2_SetWorldLocation` (`self.DefaultSceneRoot`) (`KismetMathLibrary.MakeVector` _returnvalue_x _returnvalue_y _returnvalue_z) false false)))

(event `self.Sphere.OnComponentBeginOverlap`
  (params (OverlappedComponent :type "PrimitiveComponent Object Reference") (OtherActor :type "Actor Object Reference") (OtherComp :type "PrimitiveComponent Object Reference") (OtherBodyIndex :type Integer) (bFromSweep :type Boolean) (SweepResult :type "HitResult Structure (by ref)"))
  ;[1 1 1] プレイヤーがアイテムに近づいたらインベントリに追加してアイテムのアクターを破棄
  (bind _asplayer_character (cast `/Game/2DSideScrollerBP/Blueprints/PlayerCharacter` OtherActor))
  (bind _added (`/Game/Inventory/InventoryComponent.TryAddItem` (`/Game/2DSideScrollerBP/Blueprints/PlayerCharacter.InventoryComponent` _asplayer_character) (`self.ItemObject`)))
  (if _added
    (`self.K2_DestroyActor`)))

(fn `GetDefaultItemObject`
  (returns (ItemObject :type "/Game/Items/BP_Item_Object Object Reference"))
  (return null))

(fn `GetItemObject`
  (returns (ItemObject :type "/Game/Items/BP_Item_Object Object Reference"))
  (return (`self.ItemObject`)))

(fn `UserConstructionScript`)