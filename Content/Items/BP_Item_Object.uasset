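; BP_Item_Object is the data object for a single item, with grid dimensions, icons, item class, stack count, damage, endurance and an equipment flag.
; Rotation toggles a flag that swaps the reported X/Y dimensions and selects the rotated icon.
; AddStack pours this stack into the passed item up to this item's maximum, keeping any overflow and returning true only when everything fits.
; PickOnce decrements the count without a bounds check.
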(fn `AddStack`
  (params (AddItem :type "/Game/Items/BP_Item_Object Object Reference"))
  (returns (AllStack :type Boolean))
  (bind _stacknumber (`self.StackNumber`))
  (bind _maxstucknamber (`self.MaxStuckNamber`))
  (bind _returnvalue (+ (`/Game/Items/BP_Item_Object.StackNumber` AddItem) _stacknumber))
  (if (== _stacknumber _maxstucknamber)
    (return false)
    (elif (> _returnvalue _maxstucknamber)
      (set `self.StackNumber` (- _returnvalue _maxstucknamber)) ; 最大スタック数よりも多い
      (set `/Game/Items/BP_Item_Object.StackNumber` _maxstucknamber AddItem)
      (return false)
      (else
        (set `/Game/Items/BP_Item_Object.StackNumber` _returnvalue AddItem)
        (return true)))))

(fn `GetDamage`
  (returns (Damage :type Integer))
  (return (`self.Damage`)))

(fn `GetDimensions`
  (returns (Dimensions :type "IntPoint Structure"))
  (bind (_dimensions_x _dimensions_y) (break `IntPoint` (`self.Dimensions`)))
  (if (`self.Rotated`)
    (return (make `IntPoint` _dimensions_y _dimensions_x))
    (else
      (return (`self.Dimensions`)))))

(fn `GetEndurance`
  (returns (Endurance :type Integer))
  (return (`self.Endurance`)))

(fn `GetIcon`
  (returns (Icon :type "MaterialInterface Object Reference"))
  (return (select `bool` (`self.Rotated`) :`false` (`self.Icon`) :`true` (`self.IconRotate`))))

(fn `GetIsEquipment`
  (returns (Equipment :type Boolean))
  (return (`self.Equipment`)))

(fn `GetItemClass`
  (returns (ItemClass :type "/Game/Items/BP_ItemBase Class Reference"))
  (return (`self.ItemClass`)))

(fn `GetMaxStackNumber`
  (returns (MaxStackNumber :type Integer))
  (return (`self.MaxStuckNamber`)))

(fn `GetName`
  (returns (NewParam :type Name))
  (return (`self.Name`)))

(fn `GetStackNumber`
  (returns (StackNumber :type Integer))
  (return (`self.StackNumber`)))

(fn `IsRotate`
  (returns (Rotated :type Boolean))
  (return (`self.Rotated`)))

(fn `PickOnce`
  (set `self.StackNumber` (- (`self.StackNumber`) 1)))

(fn `Rotate`
  (set `self.Rotated` (not (`self.Rotated`))))

(fn `SetEndurance`
  (params (NewParam :type Integer))
  (set `self.Endurance` NewParam)
  (return))