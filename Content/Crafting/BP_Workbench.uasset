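; Workbench actor that lets the player open a crafting UI while overlapping it.
; Overlap shows a screen-projected prompt and hands the bench's inventory component to the player.
; Tick polls the Action key to toggle the crafting widget, switching camera distance, input, cursor and crafting state.
; If closing returns equipment, an equip widget holds that state until complete; Tick also re-adds the crafting widget when crafting ends.
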(event `self.ReceiveBeginPlay`
  (bind _returnvalue (`|CreateWidget` "/Game/Box/OpenTextWidget.OpenTextWidget_C" (`GameplayStatics.GetPlayerController` 0)))
  (bind _output_get (set `self.OpenTextWidget` _returnvalue))
  (`UserWidget.AddToViewport` _output_get -100)
  (bind _returnvalue_2 (`|CreateWidget` "/Game/Crafting/CraftingWidget.CraftingWidget_C" (`GameplayStatics.GetPlayerController` 0) (`/Game/2DSideScrollerBP/Blueprints/PlayerCharacter.InventoryComponent` (cast `/Game/2DSideScrollerBP/Blueprints/PlayerCharacter` (`GameplayStatics.GetPlayerPawn` 0) :!pure true)) 50.0 0 0 (`self.InventoryComponent`)))
  (set `self.CraftingWidget` _returnvalue_2))

(event `self.ReceiveActorBeginOverlap`
  (params (OtherActor :type "Actor Object Reference"))
  (bind _opentextwidget (`self.OpenTextWidget`))
  ;[1 1 1] プレイヤーが作業台に接触した時の処理
  (if (`self.ActorHasTag` OtherActor "Player")
    (`Widget.SetVisibility` (`/Game/Box/OpenTextWidget.OpenTextBox` _opentextwidget) "SelfHitTestInvisible")
    (`UserWidget.SetPositionInViewport` _opentextwidget (`PlayerController.ProjectWorldLocationToScreen` (`GameplayStatics.GetPlayerController` 0) (`self.K2_GetActorLocation` (`GameplayStatics.GetPlayerPawn` 0)) false) true)
    (set `self.Collision` true)
    (bind _asplayer_character (cast `/Game/2DSideScrollerBP/Blueprints/PlayerCharacter` OtherActor))
    (set `/Game/2DSideScrollerBP/Blueprints/PlayerCharacter.CraftedInventoryComponent` (`self.InventoryComponent`) _asplayer_character)))

(event `self.ReceiveActorEndOverlap`
  (params (OtherActor :type "Actor Object Reference"))
  ;[1 1 1] プレイヤーが作業台から離れた時の処理
  (cast `/Game/2DSideScrollerBP/Blueprints/PlayerCharacter` OtherActor)
  (if (`self.Collision`)
    (`Widget.SetVisibility` (`/Game/Box/OpenTextWidget.OpenTextBox` (`self.OpenTextWidget`)) "Hidden")
    (set `self.Collision` false)))

(event `self.ReceiveTick`
  (params (DeltaSeconds :type "Float (single-precision)"))
  (bind _returnvalue (`GameplayStatics.GetPlayerController` 0))
  (bind _returnvalue_2 (`GameplayStatics.GetPlayerPawn` 0))
  (bind _craftingwidget (`self.CraftingWidget`))
  (bind _craftingwidget_2 (`self.CraftingWidget`))
  (bind _craftingwidget_3 (`self.CraftingWidget`))
  (bind _asplayer_character (cast `/Game/2DSideScrollerBP/Blueprints/PlayerCharacter` (`GameplayStatics.GetPlayerPawn` 0) :!pure true))
  (bind _asmain_game_pc (cast `/Game/2DSideScrollerBP/Blueprints/MainGamePC` (`GameplayStatics.GetPlayerController` 0) :!pure true))
  (bind _asmain_game_pc_2 (cast `/Game/2DSideScrollerBP/Blueprints/MainGamePC` (`GameplayStatics.GetPlayerController` 0) :!pure true))
  (bind _asmain_game_pc_3 (cast `/Game/2DSideScrollerBP/Blueprints/MainGamePC` (`GameplayStatics.GetPlayerController` 0) :!pure true))
  (bind _asmain_game_pc_4 (cast `/Game/2DSideScrollerBP/Blueprints/MainGamePC` (`GameplayStatics.GetPlayerController` 0) :!pure true))
  (`|ExecutionSequence`
    (:`then_0`
      (`/Engine/EditorBlueprintResources/StandardMacros.IsValid` (`self.Equipment`)
        (:`Is Valid`
          (`/Engine/EditorBlueprintResources/StandardMacros.IsValid` (`self.EquipWidget`)
            (:`Is Valid`
              (if (`/Game/Crafting/EquipWidget.Complete` (`self.EquipWidget`))
                (`Widget.RemoveFromParent` (`self.EquipWidget`))
                (`WidgetBlueprintLibrary.SetInputMode_GameOnly` _asmain_game_pc_4)
                (set `PlayerController.bShowMouseCursor` false _asmain_game_pc_4)
                (set `/Game/2DSideScrollerBP/Blueprints/PlayerCharacter.Crafting` false (cast `/Game/2DSideScrollerBP/Blueprints/PlayerCharacter` (`GameplayStatics.GetPlayerPawn` 0) :!pure true))
                (`Widget.RemoveFromParent` (`self.EquipWidget`))
                (`PSGamepadFunctionLibrary.DisableGamepadCursor`)
                (`self.EnableInput` (`GameplayStatics.GetPlayerPawn` 0) (`GameplayStatics.GetPlayerController` 0))
                (set `self.Equipment` null)
                (set `self.EquipWidget` null)))
            (:`Is Not Valid`
              (bind _returnvalue_3 (`|CreateWidget` "/Game/Crafting/EquipWidget.EquipWidget_C" (`GameplayStatics.GetPlayerController` 0) (`self.Equipment`)))
              (bind _output_get (set `self.EquipWidget` _returnvalue_3))
              (`UserWidget.AddToViewport` _output_get -100))))
        (:`Is Not Valid`
          (if (`self.Collision`)
            (bind _asplayer_character_2 (cast `/Game/2DSideScrollerBP/Blueprints/PlayerCharacter` (`GameplayStatics.GetPlayerPawn` 0)))
            (if (`/Game/Crafting/CraftingWidget.CraftStart` (`self.CraftingWidget`))
              (`PSGamepadFunctionLibrary.DisableGamepadCursor`)
              (else
                (bind _inputarray (`PSInputFunctionLibrary.FindCurrentActionMappings` "Action"))
                (for _array_element _inputarray
                  (if (`PlayerController.WasInputKeyJustPressed` (`GameplayStatics.GetPlayerController` 0) (`.Key` (break `PSInputWrapper` _array_element)))
                    (if (`/Game/MyGameState.OnDrag` (cast `/Game/MyGameState` (`GameplayStatics.GetGameState`) :!pure true))
                      _
                      (elif (`Widget.IsInViewport` (`self.CraftingWidget`))
                        (bind _cameraboom (`/Game/2DSideScrollerBP/Blueprints/PlayerCharacter.CameraBoom` _asplayer_character_2))
                        (set `SpringArmComponent.TargetArmLength` 400.0 _cameraboom)
                        (bind _getequipment (`/Game/Crafting/CraftingWidget.RemoveFromWorkbench` (`self.CraftingWidget`)))
                        (`/Engine/EditorBlueprintResources/StandardMacros.IsValid` _getequipment
                          (:`Is Valid`
                            (set `self.Equipment` _getequipment)
                            (`/Game/Crafting/CraftingWidget.CommandPhaseInitialize` _craftingwidget_2)
                            (`Widget.RemoveFromParent` _craftingwidget_2))
                          (:`Is Not Valid`
                            (`WidgetBlueprintLibrary.SetInputMode_GameOnly` _asmain_game_pc_2)
                            (set `PlayerController.bShowMouseCursor` false _asmain_game_pc_2)
                            (set `/Game/2DSideScrollerBP/Blueprints/PlayerCharacter.Crafting` false _asplayer_character)
                            (`/Game/Crafting/CraftingWidget.CommandPhaseInitialize` _craftingwidget_3)
                            (`Widget.RemoveFromParent` _craftingwidget_3)
                            (`PSGamepadFunctionLibrary.DisableGamepadCursor`)
                            (`self.EnableInput` _returnvalue_2 _returnvalue)))
                        (else
                          (`Widget.SetVisibility` (`/Game/Box/OpenTextWidget.OpenTextBox` (`self.OpenTextWidget`)) "Hidden")
                          (set `SpringArmComponent.TargetArmLength` 1000.0 _cameraboom)
                          (`WidgetBlueprintLibrary.SetInputMode_GameAndUIEx` _asmain_game_pc null "DoNotLock" false)
                          (set `PlayerController.bShowMouseCursor` true _asmain_game_pc)
                          (set `/Game/2DSideScrollerBP/Blueprints/PlayerCharacter.Crafting` true _asplayer_character)
                          (`UserWidget.AddToViewport` _craftingwidget_3 -100)
                          (`PSGamepadFunctionLibrary.EnableGamepadCursor`)
                          (`self.DisableInput` _returnvalue_2 _returnvalue))))))))))))
    (:`then_1`
      (if (`/Game/Crafting/CraftingWidget.CraftEnd` _craftingwidget)
        (set `/Game/Crafting/CraftingWidget.CraftEnd` false _craftingwidget)
        (`Widget.RemoveFromParent` (`self.CraftingWidget`))
        (`WidgetBlueprintLibrary.SetInputMode_GameAndUIEx` _asmain_game_pc_3 null "DoNotLock" false)
        (set `PlayerController.bShowMouseCursor` true _asmain_game_pc_3)
        (`UserWidget.AddToViewport` (`self.CraftingWidget`) -100)
        (`PSGamepadFunctionLibrary.EnableGamepadCursor`)))))

(fn `Refresh`)

(fn `UserConstructionScript`)