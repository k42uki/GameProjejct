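; BP_ItemBox is an item container that the player opens and closes with the Action input while overlapping it.
; Overlap shows an open prompt at the player's screen position and passes the box's InventoryComponent to PlayerCharacter, which is re-initialized without it on exit.
; Tick polls Action keys directly because opening disables pawn input, toggling the inventory widget, cursors and input mode unless a drag is active.
; BeginPlay pins the box to a fixed world Y.
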(event `self.ReceiveBeginPlay`
  (bind (_returnvalue_x _returnvalue_y _returnvalue_z) (`KismetMathLibrary.BreakVector` (`SceneComponent.K2_GetComponentLocation` (`self.DefaultSceneRoot`))))
  (bind _returnvalue (`|CreateWidget` "/Game/Box/OpenTextWidget.OpenTextWidget_C" (`GameplayStatics.GetPlayerController` 0)))
  (bind _output_get (set `self.OpenTextWidget` _returnvalue))
  (`UserWidget.AddToViewport` _output_get -100)
  (`SceneComponent.K2_SetWorldLocation` (`self.DefaultSceneRoot`) (`KismetMathLibrary.MakeVector` _returnvalue_x -250.0 _returnvalue_z) false false))

(event `self.ReceiveActorBeginOverlap`
  (params (OtherActor :type "Actor Object Reference"))
  (bind _opentextwidget (`self.OpenTextWidget`))
  ;[1 1 1] プレイヤーがボックスに接触した時の処理
  (if (`self.ActorHasTag` OtherActor "Player")
    (`Widget.SetVisibility` (`/Game/Box/OpenTextWidget.OpenTextBox` _opentextwidget) "SelfHitTestInvisible")
    (`UserWidget.SetPositionInViewport` _opentextwidget (`PlayerController.ProjectWorldLocationToScreen` (`GameplayStatics.GetPlayerController` 0) (`self.K2_GetActorLocation` (`GameplayStatics.GetPlayerPawn` 0)) false) true)
    (set `self.Collision` true)
    (bind _asplayer_character (cast `/Game/2DSideScrollerBP/Blueprints/PlayerCharacter` OtherActor))
    (`Widget.RemoveFromParent` (`/Game/2DSideScrollerBP/Blueprints/PlayerCharacter.InventoryWidget` _asplayer_character))
    (`/Game/2DSideScrollerBP/Blueprints/PlayerCharacter.Initialize` _asplayer_character (`self.InventoryComponent`))))

(event `self.ReceiveActorEndOverlap`
  (params (OtherActor :type "Actor Object Reference"))
  ;[1 1 1] プレイヤーがボックスから離れた時の処理
  (bind _asplayer_character (cast `/Game/2DSideScrollerBP/Blueprints/PlayerCharacter` OtherActor))
  (`/Game/2DSideScrollerBP/Blueprints/PlayerCharacter.Initialize` _asplayer_character null)
  (`Widget.SetVisibility` (`/Game/Box/OpenTextWidget.OpenTextBox` (`self.OpenTextWidget`)) "Hidden")
  (set `self.Collision` false))

(event `self.ReceiveTick`
  (params (DeltaSeconds :type "Float (single-precision)"))
  (bind _returnvalue (`GameplayStatics.GetPlayerController` 0))
  (bind _returnvalue_2 (`GameplayStatics.GetPlayerController` 0))
  (bind _returnvalue_3 (`GameplayStatics.GetPlayerPawn` 0))
  (bind _opentextbox (`/Game/Box/OpenTextWidget.OpenTextBox` (`self.OpenTextWidget`)))
  ;[1 1 1] プレイヤーがボックスを開いた時の処理
  (if (not (`/Game/MyGameState.OnDrag` (cast `/Game/MyGameState` (`GameplayStatics.GetGameState`) :!pure true)))
    ;;[1 1 1] キャラクター操作が無効になるので入力キーをこれで取得している
    (bind _inputarray (`PSInputFunctionLibrary.FindCurrentActionMappings` "Action"))
    (for _array_element _inputarray
      (if (and (`PlayerController.WasInputKeyJustPressed` (`GameplayStatics.GetPlayerController` 0) (`.Key` (break `PSInputWrapper` _array_element))) (`self.Collision`))
        (bind _asplayer_character (cast `/Game/2DSideScrollerBP/Blueprints/PlayerCharacter` _returnvalue_3))
        (bind _inventorywidget (`/Game/2DSideScrollerBP/Blueprints/PlayerCharacter.InventoryWidget` _asplayer_character))
        (if (`Widget.IsInViewport` _inventorywidget)
          (`Widget.RemoveFromParent` _inventorywidget)
          (`WidgetBlueprintLibrary.SetInputMode_GameOnly` _returnvalue)
          (set `PlayerController.bShowMouseCursor` false _returnvalue)
          (set `self.Open` false)
          (`self.EnableInput` _returnvalue_3 _returnvalue_2)
          (`Widget.SetVisibility` _opentextbox "SelfHitTestInvisible")
          (`PSGamepadFunctionLibrary.DisableGamepadCursor`)
          (else
            (`UserWidget.AddToViewport` _inventorywidget 0)
            (`WidgetBlueprintLibrary.SetInputMode_GameAndUIEx` (`GameplayStatics.GetPlayerController` 0) _inventorywidget "DoNotLock" false)
            (set `PlayerController.bShowMouseCursor` true _returnvalue_2)
            (set `self.Open` true)
            (`self.DisableInput` _returnvalue_3 _returnvalue_2) ; キャラクター操作を無効にしている
            (`Widget.SetVisibility` _opentextbox "Hidden")
            (`PSGamepadFunctionLibrary.EnableGamepadCursor`)))))))

(fn `UserConstructionScript`)